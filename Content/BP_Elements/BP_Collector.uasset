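; BP_Collector is an actor with a box volume that plays a win sound when enough components gather inside it.
; Every Tick it counts the components overlapping the Box and plays the Winbrass sound in 2D once the count reaches three or more.
; A Played flag limits the sound to once per fill and resets when the count drops below three.
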(event `self.ReceiveActorBeginOverlap`
  (params (OtherActor :type "Actor Object Reference")))

(event `self.ReceiveTick`
  (params (DeltaSeconds :type "Float (single-precision)"))
  (if (>= (`KismetArrayLibrary.Array_Length` (`PrimitiveComponent.GetOverlappingComponents` (`self.Box`))) 3)
    (if (not (`self.Played`))
      (`GameplayStatics.PlaySound2D` "/Game/Sounds/winbrass.winbrass" 1.0 1.0 0.0 null null)
      (set `self.Played` true))
    (else
      (set `self.Played` false))))

(fn `UserConstructionScript`)