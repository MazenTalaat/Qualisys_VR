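; BP_Cupboard is a cupboard with a hinged door that a motion controller can grab and swing.
; GrabDoor stores a controller within the handle sphere's radius, and ReleaseDoor clears it.
; Each tick, the look-at yaw from controller to Pivot, minus an offset and clamped, sets the pivot's relative yaw, while Highlighting toggles the door's custom depth.
; Vector-based angle and rotation helper functions are defined but unused in the event graph.
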(event `/Game/VRTemplate/Blueprints/GrabInterface.GrabDoor`
  (params (MotionController :type "MotionControllerComponent Object Reference"))
  (bind _handlecollision (`self.HandleCollision`))
  (if (== (`SceneComponent.K2_GetComponentLocation` MotionController) (`SceneComponent.K2_GetComponentLocation` _handlecollision) :`ErrorTolerance` (`SphereComponent.SphereRadius` _handlecollision))
    (set `self.Motion Controller` MotionController)))

(event `/Game/VRTemplate/Blueprints/GrabInterface.ReleaseDoor`
  (params (MotionController :type "MotionControllerComponent Object Reference"))
  (if (== MotionController (`self.Motion Controller`))
    (set `self.Motion Controller` null)))

(event `self.ReceiveTick`
  (params (DeltaSeconds :type "Float (single-precision)"))
  (bind _pivot (`self.Pivot`))
  (bind (_returnvalue_roll _returnvalue_pitch) (`KismetMathLibrary.BreakRotator` (`SceneComponent.K2_GetComponentRotation` (`self.Pivot`))))
  (`|ExecutionSequence`
    (:`then_0`
      (bind _motion_controller (`self.Motion Controller`)
        (:`then`
          (bind (_returnvalue_roll_2 _returnvalue_pitch_2 _returnvalue_yaw) (`KismetMathLibrary.BreakRotator` (`KismetMathLibrary.FindLookAtRotation` (`SceneComponent.K2_GetComponentLocation` _motion_controller) (`SceneComponent.K2_GetComponentLocation` _pivot))))
          (`SceneComponent.K2_SetRelativeRotation` _pivot (`KismetMathLibrary.MakeRotator` _returnvalue_roll _returnvalue_pitch (`KismetMathLibrary.ClampAngle` (- _returnvalue_yaw (`self.OffsetAngle`)) (`self.MinAngle`) (`self.MaxAngle`))) false false))
        (:`else`)))
    (:`then_1`
      (if (`self.Highlighting`)
        (`PrimitiveComponent.SetRenderCustomDepth` (`self.Door`) true)
        (else
          (`PrimitiveComponent.SetRenderCustomDepth` (`self.Door`) false))))))

(fn `GetDoorAngle`
  (returns (DoorAngle :type "Float (double-precision)"))
  (bind (_returnvalue_x _returnvalue_y _returnvalue_z) (`KismetMathLibrary.BreakVector` (`KismetMathLibrary.Cross_VectorVector` (`self.GetHandDoorDirection`) (`self.InitDoorDirection`))))
  (return (* (`KismetMathLibrary.DegAcos` (`KismetMathLibrary.Dot_VectorVector` (`self.GetHandDoorDirection`) (`self.InitDoorDirection`))) (`KismetMathLibrary.SelectFloat` -1.0 1.0 (< _returnvalue_z 0.0)))))

(fn `GetDoorRotation`
  (params (OptionalDirection :type "Vector Structure") (UseDirection :type Boolean))
  (returns (Rotator :type "Rotator Structure"))
  (return (`KismetMathLibrary.MakeRotFromYZ` (`KismetMathLibrary.SelectVector` OptionalDirection (`self.GetHandDoorDirection`) UseDirection) (`SceneComponent.GetUpVector` (`self.Pivot`)))))

(fn `GetHandDoorDirection`
  (returns (HandDoorDirection :type "Vector Structure"))
  (return (`KismetMathLibrary.Normal` (`KismetMathLibrary.MakeVector` (.x (- (`SceneComponent.K2_GetComponentLocation` (`self.Motion Controller`)) (`SceneComponent.K2_GetComponentLocation` (`self.Pivot`)))) (.y (- (`SceneComponent.K2_GetComponentLocation` (`self.Motion Controller`)) (`SceneComponent.K2_GetComponentLocation` (`self.Pivot`))))))))

(fn `UserConstructionScript`)